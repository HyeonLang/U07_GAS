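; BP_Cannon is a stationary turret actor that periodically fires BP_CMagicBall projectiles toward the player.
; Every tick it rotates only its Arrow component to face player pawn 0, using a look-at rotation from the actor's location.
; A looping three-second timer started on BeginPlay spawns each ball at the Arrow's world transform, so the Arrow sets both spawn point and heading.
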(event `self.ReceiveBeginPlay`
  (`KismetSystemLibrary.K2_SetTimerDelegate` (delegate `OnTimeElapsed`) 3.0 true))

(event `OnTimeElapsed`
  (`|SpawnActorFromClass` "/Game/Projectiles/BP_CMagicBall.BP_CMagicBall_C" (`SceneComponent.K2_GetComponentToWorld` (`self.Arrow`)) "Undefined" "OverrideRootScale" null null))

(event `self.ReceiveTick`
  (params (DeltaSeconds :type "Float (single-precision)"))
  (`SceneComponent.K2_SetWorldRotation` (`self.Arrow`) (`KismetMathLibrary.FindLookAtRotation` (`self.K2_GetActorLocation`) (`self.K2_GetActorLocation` (`GameplayStatics.GetPlayerPawn` 0))) false false))

(fn `UserConstructionScript`)