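; BP_Barrel_Interaction is a barrel actor that detonates by itself shortly after play begins.
; On the authority, a timer triggers Bomb, which multicasts a radial force impulse and sets a short lifespan to remove the actor.
; Interact and mesh hit events are empty.
; Explosion particle and hit-damage logic through CAttributeComponent are present but disconnected, so they never run.
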(event `self.ReceiveBeginPlay`
  (`/Engine/EditorBlueprintResources/ActorMacros.Switch Has Authority`
    (:`Authority`
      (`KismetSystemLibrary.K2_SetTimerDelegate` (delegate `Bomb`) 2.0))))

(event `Bomb`
  (`self.NetMulticast_Bomb`)
  (`self.SetLifeSpan` 2.0))

(event `NetMulticast_Bomb`
  (`RadialForceComponent.FireImpulse` (`self.RadialForce`)))

(event `CGameplayInterface.Interact`
  (params (InstigatorPawn :type "Pawn Object Reference")))

(event `self.StaticMesh.OnComponentHit`
  (params (HitComponent :type "PrimitiveComponent Object Reference") (OtherActor :type "Actor Object Reference") (OtherComp :type "PrimitiveComponent Object Reference") (NormalImpulse :type "Vector Structure") (Hit :type "HitResult Structure (by ref)")))

(fn `UserConstructionScript`)