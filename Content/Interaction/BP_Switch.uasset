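; BP_Switch is an interactable switch that triggers a linked actor and marks the interacting pawn with a key tag.
; On Interact, it tilts its handle to a fixed rotation and forwards the interaction to InteractionActor through an interface message.
; It then adds the GainKey gameplay tag to the active tags on the pawn's CActionComponent.
; The construction script tints the handle materials from HandleColor.
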(event `CGameplayInterface.Interact`
  (params (InstigatorPawn :type "Pawn Object Reference"))
  (`SceneComponent.K2_SetRelativeRotation` (`self.Handle`) (struct :`Pitch` -30.0) false false)
  (message `CGameplayInterface.Interact` (`self.InteractionActor`) InstigatorPawn)
  (`BlueprintGameplayTagLibrary.AddGameplayTag` (`CActionComponent.ActiveGamePlayTags` (`self.GetComponentByClass` InstigatorPawn "/Script/GAS.CActionComponent")) (`self.GainKey`)))

(fn `UserConstructionScript`
  (`MeshComponent.SetVectorParameterValueOnMaterials` (`self.Handle`) "Color" (`KismetMathLibrary.Conv_LinearColorToVector` (`self.HandleColor`))))