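; BP_SavePoint is an interactable save point with a fire particle effect.
; Each Interact flips the FireActive flag, activating or deactivating the particle system to match.
; When the flag turns on, it calls WriteSaveGame on CGameMode and prints a debug message.
; OnActorLoaded runs the same toggle, so it inverts the current flag rather than reapplying it.
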(event `CGameplayInterface.Interact`
  (params (InstigatorPawn :type "Pawn Object Reference"))
  (`self.FireActive`)
  (if (`self.bFireActive`)
    (bind _ascgame_mode (cast `CGameMode` (`GameplayStatics.GetGameMode`)))
    (`CGameMode.WriteSaveGame` _ascgame_mode)
    (`KismetSystemLibrary.PrintString` "SaveGame")))

(event `FireActive`
  (bind _particlesystem (`self.ParticleSystem`))
  (bind _output_get (set `self.bFireActive` (not (`self.bFireActive`))))
  (if _output_get
    (`ActorComponent.Activate` _particlesystem false)
    (else
      (`ActorComponent.Deactivate` _particlesystem))))

(event `CGameplayInterface.OnActorLoaded`
  (`self.FireActive`))

(fn `UserConstructionScript`)